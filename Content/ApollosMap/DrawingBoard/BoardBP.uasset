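; Chalkboard actor that players can draw on by painting into a render target.
; On BeginPlay it creates a dynamic chalk material instance, clears BoardRT to black and registers itself as the Board on GameModeBP.
; DrawOnBoard passes a 2D location into the material's DrawLocation parameter and draws that material onto the render target, adding a chalk stroke at that point.
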(event `self.ReceiveBeginPlay`
  (bind _returnvalue (`KismetMaterialLibrary.CreateDynamicMaterialInstance` "/Game/ApollosMap/DrawingBoard/ChalkMaterial.ChalkMaterial"))
  (set `self.ChalkMaterialMatInstance` _returnvalue)
  (`KismetRenderingLibrary.ClearRenderTarget2D` "/Game/ApollosMap/DrawingBoard/BoardRT.BoardRT")
  (set `/Game/ApollosMap/GameModeBP.Board` self (cast `/Game/ApollosMap/GameModeBP` (`GameplayStatics.GetGameMode`) :!pure true)))

(event `Draw On Board`
  (params (`Location To Draw` :type "Vector2D Structure"))
  (`MaterialInstanceDynamic.SetVectorParameterValue` (`self.ChalkMaterialMatInstance`) "DrawLocation" (`KismetMathLibrary.Conv_VectorToLinearColor` (`KismetMathLibrary.Conv_Vector2DToVector` `Location To Draw`)))
  (`KismetRenderingLibrary.DrawMaterialToRenderTarget` "/Game/ApollosMap/DrawingBoard/BoardRT.BoardRT" (`self.ChalkMaterialMatInstance`)))

(fn `UserConstructionScript`)