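; Player controller for the drawing board map, currently inactive: BeginPlay and SendDrawDatatoBoard are empty.
; Disconnected nodes would create a viewport widget and call DrawOnBoard at a zero position on the game mode's board.
; They also contain an unused mouse-to-world visibility trace that would pass the hit's collision UV to BoardBP for drawing.
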(event `self.ReceiveBeginPlay`)

(event `self.SendDrawDataToBoard`
  (params (UV :type "Vector2D Structure")))

(fn `UserConstructionScript`)