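; Procedurally randomized planet actor that orbits a center actor or point and can spawn its own MoonBP satellites.
; Construction picks mesh, tinted dynamic materials, scale and occasional belts or rings, taking the owner's location as center.
; BeginPlay occasionally spawns moons centered on the planet.
; Tick re-orthogonalizes the orbit axis, rotates the planet's offset around it and spins the belts; the stored previous center never updates after BeginPlay.
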(event `OrthogonalizeAxis`
  (bind _returnvalue (- (`self.K2_GetActorLocation`) (`self.CenterLocation`)))
  (set `self.Axis` (`KismetMathLibrary.Normal` (`KismetMathLibrary.Cross_VectorVector` _returnvalue (`KismetMathLibrary.Cross_VectorVector` (`self.Axis`) _returnvalue)))))

(event `self.ReceiveBeginPlay`
  (if (== 1 (`KismetMathLibrary.RandomIntegerInRange` 1 5))
    (`self.SpawnMoons`))
  (`|ExecutionSequence`
    (:`then_0`
      (bind _centeractor (`self.CenterActor`)
        (:`then`
          (set `self.CenterLocation` (`self.K2_GetActorLocation` _centeractor)))
        (:`else`)))
    (:`then_1`
      (set `self.OldCenterVariable` (`self.CenterLocation`)))))

(event `self.ReceiveTick`
  (params (DeltaSeconds :type "Float (single-precision)"))
  (`|ExecutionSequence`
    (:`then_0`
      (bind _centeractor (`self.CenterActor`)
        (:`then`
          (set `self.CenterLocation` (`self.K2_GetActorLocation` _centeractor)))
        (:`else`)))
    (:`then_1`
      (`self.OrthogonalizeAxis`)
      (`self.K2_SetActorLocation` (+ (`KismetMathLibrary.RotateAngleAxis` (- (`self.K2_GetActorLocation`) (`self.OldCenterVariable`)) (* DeltaSeconds (`self.Speed`)) (`self.Axis`)) (`self.CenterLocation`)))
      (set `self.OldCenterVariable` (`self.OldCenterVariable`))
      (`SceneComponent.K2_AddLocalRotation` (`self.BeltsOrRings`) (* (`KismetMathLibrary.MakeRotator` 0.0 0.0 (`self.BeltsRotationSpeed`)) DeltaSeconds) false false))))

(fn `SetCenterLocation`
  (params (CenterVector :type "Vector Structure"))
  (set `self.CenterLocation` CenterVector))

(fn `SetMaterialColorGround`
  (params (Material :type "MaterialInstanceDynamic Object Reference"))
  (returns (MaterialOutput :type "MaterialInstanceDynamic Object Reference"))
  (locals (DynamicMaterial :type "MaterialInstanceDynamic Object Reference"))
  (bind _output_get (set `local.DynamicMaterial` Material))
  (`MaterialInstanceDynamic.SetVectorParameterValue` _output_get "Color Tint" (make `LinearColor` (`KismetMathLibrary.RandomFloatInRange` 0.0 1.0) (`KismetMathLibrary.RandomFloatInRange` 0.0 1.0) (`KismetMathLibrary.RandomFloatInRange` 0.0 1.0) 1.0))
  (return (`local.DynamicMaterial`)))

(fn `SetMaterialColorMountians`
  (params (Material :type "MaterialInstanceDynamic Object Reference"))
  (returns (MaterialOutput :type "MaterialInstanceDynamic Object Reference"))
  (locals (DynamicMaterial :type "MaterialInstanceDynamic Object Reference"))
  (bind _output_get (set `local.DynamicMaterial` Material))
  (`MaterialInstanceDynamic.SetVectorParameterValue` _output_get "Color Tint" (make `LinearColor` (`KismetMathLibrary.RandomFloatInRange` 0.0 1.0) (`KismetMathLibrary.RandomFloatInRange` 0.0 1.0) (`KismetMathLibrary.RandomFloatInRange` 0.0 1.0) 1.0))
  (return (`local.DynamicMaterial`)))

(fn `SpawnMoons`
  (bind _returnvalue (`KismetMathLibrary.MakeTransform` (`KismetMathLibrary.MakeVector` (`KismetMathLibrary.SelectFloat` (`KismetMathLibrary.RandomFloatInRange` 30.0 70.0) (`KismetMathLibrary.RandomFloatInRange` -30.0 -70.0) (`KismetMathLibrary.RandomBool`)) (`KismetMathLibrary.SelectFloat` (`KismetMathLibrary.RandomFloatInRange` 30.0 70.0) (`KismetMathLibrary.RandomFloatInRange` -30.0 -70.0) (`KismetMathLibrary.RandomBool`)) (`KismetMathLibrary.SelectFloat` (`KismetMathLibrary.RandomFloatInRange` 30.0 70.0) (`KismetMathLibrary.RandomFloatInRange` -30.0 -70.0) (`KismetMathLibrary.RandomBool`))) (.rotation (`self.GetTransform`)) (.scale (`self.GetTransform`))))
  (if (== 1 (`KismetMathLibrary.RandomIntegerInRange` 1 5))
    (for _ (range 1 (+ (`KismetMathLibrary.RandomIntegerInRange` 2 7) 1))
      (bind _returnvalue_2 (`|SpawnActorFromClass` "/Game/ApollosMap/CelestialBodies/MoonBP.MoonBP_C" _returnvalue "Undefined" "OverrideRootScale" self null))
      (set `/Game/ApollosMap/CelestialBodies/MoonBP.CenterActor` self _returnvalue_2))
    (else
      (bind _returnvalue_3 (`|SpawnActorFromClass` "/Game/ApollosMap/CelestialBodies/MoonBP.MoonBP_C" _returnvalue "Undefined" "OverrideRootScale" self null))
      (set `/Game/ApollosMap/CelestialBodies/MoonBP.CenterActor` self _returnvalue_3))))

(fn `UserConstructionScript`
  (locals (PlanetMeshesArray :type "Array of StaticMesh Object Reference") (PlanetMaterialsArray :type "Array of MaterialInstance Object Reference") (DynamicMaterial :type "MaterialInstanceDynamic Object Reference") (DynamicMaterialMountains :type "MaterialInstanceDynamic Object Reference") (WaterAndLavaMaterialsArray :type "Array of MaterialInstance Object Reference") (BeltsAndRingsMeshesArray :type "Array of StaticMesh Object Reference") (BeltsAndRingsMaterialsArray :type "Array of MaterialInstance Object Reference"))
  (bind _beltsorrings (`self.BeltsOrRings`))
  (bind _returnvalue (`KismetMathLibrary.FClamp` (`KismetMathLibrary.RandomFloat`) 0.01 0.2))
  (`self.SetCenterLocation` (`self.K2_GetActorLocation` (`self.GetOwner`)))
  (set `self.Speed` (`KismetMathLibrary.FClamp` (`KismetMathLibrary.RandomFloat`) 3.0 10.0))
  (`StaticMeshComponent.SetStaticMesh` (`self.Planet`) (`|GetArrayItem` (`local.PlanetMeshesArray`) (`KismetMathLibrary.RandomIntegerInRange` 0 99)))
  (bind _returnvalue_2 (`KismetMaterialLibrary.CreateDynamicMaterialInstance` (`|GetArrayItem` (`local.WaterAndLavaMaterialsArray`) (`KismetMathLibrary.RandomIntegerInRange` 0 8))))
  (bind _output_get (set `local.DynamicMaterial` _returnvalue_2))
  (bind _materialoutput (`self.SetMaterialColorGround` _output_get))
  (bind _output_get_2 (set `local.DynamicMaterial` _materialoutput))
  (`self.SetMaterialColorMountians` _output_get_2)
  (bind _returnvalue_3 (`KismetMaterialLibrary.CreateDynamicMaterialInstance` (`|GetArrayItem` (`local.PlanetMaterialsArray`) (`KismetMathLibrary.RandomIntegerInRange` 0 11))))
  (set `local.DynamicMaterialMountains` _returnvalue_3)
  (`PrimitiveComponent.SetMaterial` (`self.Planet`) 0 (`local.DynamicMaterial`))
  (`PrimitiveComponent.SetMaterial` (`self.Planet`) 1 (`local.DynamicMaterialMountains`))
  (`SceneComponent.SetWorldScale3D` (`self.Planet`) (`KismetMathLibrary.MakeVector` _returnvalue _returnvalue _returnvalue))
  (if (== (`KismetMathLibrary.RandomIntegerInRange` 1 5) 1)
    (`StaticMeshComponent.SetStaticMesh` _beltsorrings (`KismetArrayLibrary.Array_Random` (`local.BeltsAndRingsMeshesArray`)))
    (`PrimitiveComponent.CreateDynamicMaterialInstance` _beltsorrings 0 (`KismetArrayLibrary.Array_Random` (`local.BeltsAndRingsMaterialsArray`)) "None")
    (`SceneComponent.SetWorldScale3D` _beltsorrings (`KismetMathLibrary.Conv_DoubleToVector` (`KismetMathLibrary.RandomFloatInRange` 0.01 1.0)))))