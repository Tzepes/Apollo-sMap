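; MoonBP is a celestial body that orbits a CenterActor, following it as it moves.
; Each tick it re-orthogonalizes the orbit axis against the radius with a double cross product, then rotates the previous-frame offset around that axis and adds the current center location.
; The construction script randomizes body scale and sets orbit speed, though clamping a 0–1 random float to a higher range makes speed constant.
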(event `Orthogonalize Axis`
  (bind _returnvalue (- (`self.K2_GetActorLocation`) (`self.CenterLocation`)))
  (set `self.Axis` (`KismetMathLibrary.Normal` (`KismetMathLibrary.Cross_VectorVector` _returnvalue (`KismetMathLibrary.Cross_VectorVector` (`self.Axis`) _returnvalue)))))

(event `self.ReceiveBeginPlay`
  (`|ExecutionSequence`
    (:`then_0`
      (bind _centeractor (`self.CenterActor`)
        (:`then`
          (set `self.CenterLocation` (`self.K2_GetActorLocation` _centeractor)))
        (:`else`)))
    (:`then_1`
      (set `self.OldCenterLocation` (`self.CenterLocation`)))))

(event `self.ReceiveTick`
  (params (DeltaSeconds :type "Float (single-precision)"))
  (`|ExecutionSequence`
    (:`then_0`
      (bind _centeractor (`self.CenterActor`)
        (:`then`
          (set `self.CenterLocation` (`self.K2_GetActorLocation` _centeractor)))
        (:`else`)))
    (:`then_1`
      (`self.Orthogonalize Axis`)
      (`self.K2_SetActorLocation` (+ (`KismetMathLibrary.RotateAngleAxis` (- (`self.K2_GetActorLocation`) (`self.OldCenterLocation`)) (* DeltaSeconds (`self.Speed`)) (`self.Axis`)) (`self.CenterLocation`)))
      (set `self.OldCenterLocation` (`self.CenterLocation`)))))

(fn `SetCenterLocation`
  (params (CenterVector :type "Vector Structure"))
  (set `self.CenterLocation` CenterVector))

(fn `UserConstructionScript`
  (bind _centeractor (`self.CenterActor`))
  (set `self.Speed` (/ (`KismetMathLibrary.FClamp` (`KismetMathLibrary.RandomFloat`) 30.0 100.0) 2.0))
  (`SceneComponent.SetWorldScale3D` (`self.Body`) (`KismetMathLibrary.Conv_DoubleToVector` (`KismetMathLibrary.RandomFloatInRange` 0.05 0.1)))
  (if (not (== _centeractor null))
    (`self.SetCenterLocation` (`self.K2_GetActorLocation` _centeractor))))