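; StarBP is a star actor that randomizes its look and spawns its own planets at BeginPlay.
; It applies a random entry from StarMaterials to Body, then tints StarLighting with that material's "Color" parameter so the light matches the surface.
; It then spawns a random handful of PlanetBP actors, owned by the star, at small random offsets from its location, which is randomly negated.
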(event `self.ReceiveBeginPlay`
  (`PrimitiveComponent.CreateDynamicMaterialInstance` (`self.Body`) 0 (`KismetArrayLibrary.Array_Random` (`self.StarMaterials`)) "None")
  (`self.StarLight`)
  (for _ (range (+ (`KismetMathLibrary.RandomInteger` 7) 1))
    (`|SpawnActorFromClass` "/Game/ApollosMap/CelestialBodies/PlanetBP.PlanetBP_C" (`KismetMathLibrary.MakeTransform` (+ (`KismetMathLibrary.MakeVector` (* 1000.0 (`KismetMathLibrary.FClamp` (`KismetMathLibrary.RandomFloat`) -1000.0 1000.0)) (* 1000.0 (`KismetMathLibrary.FClamp` (`KismetMathLibrary.RandomFloat`) -1000.0 1000.0)) (* 1000.0 (`KismetMathLibrary.FClamp` (`KismetMathLibrary.RandomFloat`) -1000.0 1000.0))) (* (.location (`self.GetTransform`)) (`KismetMathLibrary.SelectInt` 1 -1 (== (`KismetMathLibrary.RandomBool`) false)))) (.rotation (`self.GetTransform`)) (.scale (`self.GetTransform`))) "Undefined" "OverrideRootScale" self null)))

(fn `StarLight`
  (`self.StarLightColor` (`PrimitiveComponent.GetMaterial` (`self.Body`) 0)))

(fn `StarLightColor`
  (params (SourceMaterial :type "MaterialInterface Object Reference"))
  (bind _returnvalue (`PrimitiveComponent.CreateDynamicMaterialInstance` (`self.Body`) 0 SourceMaterial "None"))
  (bind _returnvalue_2 (`MaterialInstanceDynamic.K2_GetVectorParameterValue` _returnvalue "Color"))
  (bind _output_get (set `self.StarLighting` (`self.StarLighting`)))
  (`LightComponent.SetLightColor` _output_get _returnvalue_2 true))

(fn `UserConstructionScript`)