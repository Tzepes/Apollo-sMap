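; Horizontal lever Blueprint for the telescope in ApollosMap, a child class that overrides MoveTelescope to drive the telescope's horizontal element.
; It calls the parent, gets TelescopeHorizontalElement from GameModeBP and passes it a rotation built from its current one, with an addition on yaw only.
; AxisInput is unused: both the parent call and the yaw offset receive zero, so the rotation passed on is unchanged.
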(fn `MoveTelescope`
  (params (`Axis Input` :type "Float (double-precision)"))
  (returns (Amount :type "Float (double-precision)"))
  (bind _telescope_horizontal_element (`/Game/ApollosMap/GameModeBP.Telescope Horizontal Element` (cast `/Game/ApollosMap/GameModeBP` (`GameplayStatics.GetGameMode`) :!pure true)))
  (bind _amount (`parent.MoveTelescope` 0.0))
  (`/Game/ApollosMap/Observatory/DomeAndTelescope/DomeAndTelescope_ElementBaseBP.Pass Input Rotation` _telescope_horizontal_element (`KismetMathLibrary.MakeRotator` (.roll (`self.K2_GetActorRotation` _telescope_horizontal_element)) (.pitch (`self.K2_GetActorRotation` _telescope_horizontal_element)) (+ 0.0 (.yaw (`self.K2_GetActorRotation` _telescope_horizontal_element)))))
  (return _amount))

(fn `UserConstructionScript`
  (`parent.UserConstructionScript`))