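; Lever Blueprint in ApollosMap, apparently intended to steer the telescope's vertical element while toggled into interaction.
; While interacting, Tick rolls the lever mesh by the magnitude of two input axes.
; MoveTelescope fetches the telescope element through GameModeBP and passes back its current roll and pitch with zero yaw.
; The axis input is only returned for the lever's roll, never added to the telescope's rotation.
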(event `self.ReceiveTick`
  (params (DeltaSeconds :type "Float (single-precision)"))
  (if (`self.IsInteracting`)
    (bind _amount (`self.MoveTelescope` (`KismetMathLibrary.VSize2D` (`KismetMathLibrary.MakeVector2D` (`self.GetInputAxisKeyValue`) (`self.GetInputAxisKeyValue`)))))
    (`SceneComponent.K2_AddLocalRotation` (`self.StaticMeshComponent`) (`KismetMathLibrary.MakeRotator` _amount) false false)))

(fn `InteractToggle`
  (set `self.IsInteracting` (not (`self.IsInteracting`))))

(fn `MoveTelescope`
  (params (`Axis Input` :type "Float (double-precision)"))
  (returns (Amount :type "Float (double-precision)"))
  (bind _telescope_vertical_element (`/Game/ApollosMap/GameModeBP.Telescope Vertical Element` (cast `/Game/ApollosMap/GameModeBP` (`GameplayStatics.GetGameMode`) :!pure true)))
  (`/Game/ApollosMap/Observatory/DomeAndTelescope/DomeAndTelescope_ElementBaseBP.Pass Input Rotation` _telescope_vertical_element (`KismetMathLibrary.MakeRotator` (.roll (`self.K2_GetActorRotation` _telescope_vertical_element)) (+ 0.0 (.pitch (`self.K2_GetActorRotation` _telescope_vertical_element)))))
  (return `Axis Input`))

(fn `UserConstructionScript`)