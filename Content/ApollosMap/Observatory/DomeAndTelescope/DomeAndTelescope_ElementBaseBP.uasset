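; Base Blueprint for rotatable elements of the observatory dome and telescope in Apollo's map.
; PassInputRotation stores a target rotation and starts rotating.
; Tick interpolates the actor's rotation toward that target with RInterpTo at RotationSpeed, then stops once it is within a small tolerance.
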(event `self.ReceiveTick`
  (params (DeltaSeconds :type "Float (single-precision)"))
  (if (`self.IsRotating`)
    (`self.K2_SetActorRotation` (`KismetMathLibrary.RInterpTo` (`self.K2_GetActorRotation`) (`self.IntendedRotation`) DeltaSeconds (`self.RotationSpeed`)))
    (if (== (`self.K2_GetActorRotation`) (`self.IntendedRotation`) :`ErrorTolerance` 0.1)
      (set `self.IsRotating` false))))

(fn `Pass Input Rotation`
  (params (Rotation :type "Rotator Structure"))
  (set `self.IntendedRotation` Rotation)
  (if (not (`self.IsRotating`))
    (set `self.IsRotating` true)))

(fn `UserConstructionScript`)