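; Base actor Blueprint for rotating elements of the observatory telescope.
; PassInputRotation stores a target rotation, but its IsRotating branch only writes false, so nothing here starts motion.
; While IsRotating is true, Tick lerps from the current rotation toward the target by DeltaSeconds times RotationSpeed.
; The lerp result is applied as an added local rotation delta rather than set as the absolute rotation.
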(event `self.ReceiveTick`
  (params (DeltaSeconds :type "Float (single-precision)"))
  (if (`self.IsRotating`)
    (`self.K2_AddActorLocalRotation` (`KismetMathLibrary.RLerp` (`self.K2_GetActorRotation`) (`self.IntendedRotation`) (* DeltaSeconds (`self.RotationSpeed`))))))

(fn `Pass Input Rotation`
  (params (Rotation :type "Rotator Structure"))
  (set `self.IntendedRotation` Rotation)
  (if (not (`self.IsRotating`))
    (set `self.IsRotating` false)))

(fn `UserConstructionScript`)